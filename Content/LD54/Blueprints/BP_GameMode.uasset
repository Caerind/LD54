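; Game mode for a PC-building puzzle: runs the level loop, spawns the casing and parts, and tracks unlocks and money.
; OnPieceChanged totals validly placed pieces' performance, heat and wattage, applying same-vendor motherboard boosts, then updates the machine-state UI and gates launching on level requirements and limits.
; Launch pays out piece prices, clears the board, unlocks parts and shows the economy screen.
; StartLevel loads the next LevelLib entry or the game-end widget.
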(event `self.ReceiveBeginPlay`
  (`self.Init`)
  (`self.StartLevel`))

(fn `ClearLevel`
  (bind _pieces (`self.Pieces`))
  (bind _newpiece (`self.NewPiece`))
  (for _array_element _pieces
    (`self.K2_DestroyActor` _array_element))
  (`KismetArrayLibrary.Array_Clear` _pieces)
  (`self.K2_DestroyActor` (`self.Casing`))
  (set `self.Casing` null)
  (`/Engine/EditorBlueprintResources/StandardMacros.IsValid` _newpiece
    (:`Is Valid`
      (`self.K2_DestroyActor` _newpiece))
    (:`Is Not Valid`
      _))
  (`self.OnPieceChanged` null))

(fn `GetHeatForPiece`
  (params (PieceData :type "/Game/LD54/Blueprints/Structures/PieceData Structure"))
  (returns (Heat :type Integer))
  (return (* PieceData_Watt_12_137A27F7408F5A7090CBB5ACEC276EED (`KismetArrayLibrary.Array_Length` PieceData_PieceShape_32_2D49CDF54DD6A031E99A61B5D860E5B7))))

(fn `GetPerformanceForType`
  (params (PieceType :type "/Game/LD54/Blueprints/Structures/PieceType Enum" :default "NewEnumerator0"))
  (returns (Performance :type Integer))
  (locals (Result :type Integer))
  (set `local.Result` 0)
  (for _array_element (`self.Pieces`)
    (bind (_piecedata_name _piecedata_vendor _piecedata_piecetype _piecedata_pieceshape _piecedata_performance) (break `/Game/LD54/Blueprints/Structures/PieceData` (`/Game/LD54/Blueprints/BP_Piece.PieceData` _array_element)))
    (if (and (`|EnumEquality` PieceType _piecedata_piecetype) (`/Game/LD54/Blueprints/BP_Piece.ValidPos` _array_element))
      (set `local.Result` (+ (`local.Result`) _piecedata_performance))))
  (return (`local.Result`)))

(fn `GetPriceForPiece`
  (params (Piece :type "/Game/LD54/Blueprints/Structures/PieceData Structure"))
  (returns (Price :type Integer))
  (bind _returnvalue (`KismetArrayLibrary.Array_Length` Piece_PieceShape_32_2D49CDF54DD6A031E99A61B5D860E5B7))
  (return (+ (* _returnvalue _returnvalue 1) (`KismetMathLibrary.Abs_Int` Piece_Performance_10_B982DDF74F67336160DD05AA7A1CE159) (* _returnvalue -2) 5)))

(fn `GetRequirementForType`
  (params (PieceType :type "/Game/LD54/Blueprints/Structures/PieceType Enum" :default "NewEnumerator0"))
  (returns (Requirement :type Integer))
  (locals (req :type Integer))
  (bind (_currentleveldata_casing _currentleveldata_requirements) (break `/Game/LD54/Blueprints/Structures/LevelData` (`self.CurrentLevelData`)))
  (set `local.req` 0)
  (for _array_element _currentleveldata_requirements
    (if (`|EnumEquality` (break `/Game/LD54/Blueprints/Structures/Requirement` _array_element) PieceType)
      (set `local.req` (+ (`local.req`) (`.Performance_6_1EDF2D8E40A049E2705FFC901E1A8807` (break `/Game/LD54/Blueprints/Structures/Requirement` _array_element))))))
  (return (`local.req`)))

(fn `GetUnlockedPieceDataForType`
  (params (PieceType :type "/Game/LD54/Blueprints/Structures/PieceType Enum" :default "NewEnumerator0"))
  (returns (PieceData :type "Array of /Game/LD54/Blueprints/Structures/PieceData Structure"))
  (locals (Result :type "Array of /Game/LD54/Blueprints/Structures/PieceData Structure"))
  (for _array_element (`self.UnlockedPieces`)
    (if (`|EnumEquality` PieceType (`.PieceType_28_0167DE8540C229F3F3ABC6A354513B2D` (break `/Game/LD54/Blueprints/Structures/PieceData` _array_element)))
      (`KismetArrayLibrary.Array_Add` (`local.Result`) _array_element)))
  (return (`local.Result`)))

(fn `Init`
  (bind _returnvalue (`|CreateWidget` "/Game/LD54/Blueprints/UI/Eco/WBP_ECO.WBP_ECO_C"))
  (set `self.EcoUI` _returnvalue)
  (bind _returnvalue_2 (`|CreateWidget` "/Game/LD54/Blueprints/UI/Hints/WBP_Hints.WBP_Hints_C"))
  (`UserWidget.AddToViewport` _returnvalue_2 0)
  (bind _returnvalue_3 (`|CreateWidget` "/Game/LD54/Blueprints/UI/LaunchUI/WBP_LaunchUI.WBP_LaunchUI_C"))
  (bind _output_get (set `self.LaunchUI` _returnvalue_3))
  (`UserWidget.AddToViewport` _output_get 0)
  (bind _returnvalue_4 (`|CreateWidget` "/Game/LD54/Blueprints/UI/BreakingNewsUI/WBP_BreakingNews.WBP_BreakingNews_C"))
  (bind _output_get_2 (set `self.BreakingNewsUI` _returnvalue_4))
  (`UserWidget.AddToViewport` _output_get_2 0)
  (bind _returnvalue_5 (`|CreateWidget` "/Game/LD54/Blueprints/UI/MachineStateUI/WBP_MachineState.WBP_MachineState_C"))
  (bind _output_get_3 (set `self.MachineStateUI` _returnvalue_5))
  (`UserWidget.AddToViewport` _output_get_3 0)
  (bind _returnvalue_6 (`|GenericCreateObject` "/Game/LD54/Data/LevelLib.LevelLib_C"))
  (set `self.LevelLib` _returnvalue_6)
  (bind _returnvalue_7 (`|GenericCreateObject` "/Game/LD54/Data/PieceLib.PieceLib_C"))
  (set `self.PieceLib` _returnvalue_7)
  ;[1 1 1] Unlock pieces
  (for _array_element (`/Game/LD54/Data/PieceLib.Pieces` (`self.PieceLib`))
    (bind (_name _vendor _piecetype _pieceshape _performance _watt _sprite _texturesize _unlockedlevel) (break `/Game/LD54/Blueprints/Structures/PieceData` _array_element))
    (if (or (`self.UnlockAllCheat`) (and (>= _unlockedlevel 0) (<= _unlockedlevel (+ (`self.CurrentLevelIndex`) 1))))
      (`KismetArrayLibrary.Array_AddUnique` (`self.UnlockedPieces`) _array_element)))
  (`self.OnPieceChanged` null))

(fn `Launch`
  (locals (HasUnlockedPiece :type Boolean) (UnlockedPieceData :type "/Game/LD54/Blueprints/Structures/PieceData Structure") (Gain :type Integer))
  (if (`self.CanLaunch`)
    ;[1 1 1] Gain
    (for _array_element (`self.Pieces`)
      (set `local.Gain` (+ (`local.Gain`) (`self.GetPriceForPiece` (`/Game/LD54/Blueprints/BP_Piece.PieceData` _array_element)))))
    (set `self.Balance` (+ (`local.Gain`) (`self.Balance`)))
    (`self.ClearLevel`)
    ;[1 1 1] Unlock pieces
    (for _array_element_2 (`/Game/LD54/Data/PieceLib.Pieces` (`self.PieceLib`))
      (if (== (`.UnlockedLevel_37_9D3344A347DF7928F241FAAA6682C1AD` (break `/Game/LD54/Blueprints/Structures/PieceData` _array_element_2)) (+ (`self.CurrentLevelIndex`) 1))
        (`KismetArrayLibrary.Array_AddUnique` (`self.UnlockedPieces`) _array_element_2)
        (set `local.UnlockedPieceData` _array_element_2)
        (set `local.HasUnlockedPiece` true)))
    ;[1 1 1] UI
    (`/Game/LD54/Blueprints/UI/Eco/WBP_ECO.FinishLevel` (`self.EcoUI`) (`local.Gain`) (`self.Balance`) (`local.UnlockedPieceData`) (`local.HasUnlockedPiece`))
    (`UserWidget.AddToViewport` (`self.EcoUI`) 0)))

(fn `OnPieceChanged`
  (params (Piece :type "/Game/LD54/Blueprints/BP_Piece Object Reference"))
  (locals (Motherboards :type "Map of /Game/LD54/Blueprints/Structures/Vendor Enum to Integer") (TotalHeat :type Integer) (CPU :type Integer) (GPU :type Integer) (RAM :type Integer) (DISK :type Integer) (TempMotherboard :type Integer) (TempBoost :type "Float (double-precision)") (CPUBoosted :type Boolean) (GPUBoosted :type Boolean) (RAMBoosted :type Boolean) (DISKBoosted :type Boolean) (MaxWatt :type Integer) (MaxWattBoosted :type Boolean) (TotalWatt :type Integer) (HeatReducBoosted :type Boolean))
  (bind (_currentleveldata_casing _currentleveldata_requirements) (break `/Game/LD54/Blueprints/Structures/LevelData` (`self.CurrentLevelData`)))
  (bind _motherboards (`local.Motherboards`))
  (bind _motherboards_2 (`local.Motherboards`))
  (bind _newpiece (`self.NewPiece`))
  (bind _returnvalue (> (`local.TempBoost`) 1.0))
  ;[1 1 1] New Piece Management
  (`/Engine/EditorBlueprintResources/StandardMacros.IsValid` _newpiece
    (:`Is Valid`
      (if (== Piece _newpiece)
        (`KismetArrayLibrary.Array_AddUnique` (`self.Pieces`) _newpiece)
        (set `self.NewPiece` null)))
    (:`Is Not Valid`
      _))
  ;[1 1 1] Init
  (`BlueprintMapLibrary.Map_Clear` (`local.Motherboards`))
  (set `local.TotalHeat` 0)
  (set `local.CPU` 0)
  (set `local.GPU` 0)
  (set `local.RAM` 0)
  (set `local.DISK` 0)
  (set `local.CPUBoosted` false)
  (set `local.GPUBoosted` false)
  (set `local.RAMBoosted` false)
  (set `local.DISKBoosted` false)
  (set `local.MaxWatt` 0)
  (set `local.MaxWattBoosted` false)
  (set `local.TotalWatt` 0)
  (set `local.HeatReducBoosted` false)
  ;[1 1 1] Compute Motherboards
  (for _array_element (`self.Pieces`)
    (bind (_piecedata_name _piecedata_vendor _piecedata_piecetype _piecedata_pieceshape _piecedata_performance) (break `/Game/LD54/Blueprints/Structures/PieceData` (`/Game/LD54/Blueprints/BP_Piece.PieceData` _array_element)))
    (if (and (`KismetSystemLibrary.IsValid` _array_element) (`|EnumEquality` _piecedata_piecetype "NewEnumerator0") (`/Game/LD54/Blueprints/BP_Piece.ValidPos` _array_element))
      (if (`BlueprintMapLibrary.Map_Contains` _motherboards _piecedata_vendor)
        (set `local.TempMotherboard` (+ (`BlueprintMapLibrary.Map_Find` _motherboards _piecedata_vendor) _piecedata_performance))
        (`BlueprintMapLibrary.Map_Remove` _motherboards _piecedata_vendor)
        (`BlueprintMapLibrary.Map_Add` _motherboards _piecedata_vendor (`local.TempMotherboard`))
        (else
          (`BlueprintMapLibrary.Map_Add` _motherboards _piecedata_vendor _piecedata_performance)))))
  (for _array_element_2 (`self.Pieces`)
    (if (and (`KismetSystemLibrary.IsValid` _array_element_2) (`/Game/LD54/Blueprints/BP_Piece.ValidPos` _array_element_2))
      (bind (_piecedata_name_2 _piecedata_vendor_2 _piecedata_piecetype_2 _piecedata_pieceshape_2 _piecedata_performance_2 _piecedata_watt) (break `/Game/LD54/Blueprints/Structures/PieceData` (`/Game/LD54/Blueprints/BP_Piece.PieceData` _array_element_2)))
      (if (and (`|EnumInequality` _piecedata_piecetype_2 "NewEnumerator0") (`BlueprintMapLibrary.Map_Contains` _motherboards_2 _piecedata_vendor_2))
        (set `local.TempBoost` (+ (* (`BlueprintMapLibrary.Map_Find` _motherboards_2 _piecedata_vendor_2) 0.01) 1.0))
        (else
          (set `local.TempBoost` 1.0)))
      (set `local.TotalWatt` (+ _piecedata_watt (`local.TotalWatt`)))
      (set `local.TotalHeat` (+ (`self.GetHeatForPiece` (`/Game/LD54/Blueprints/BP_Piece.PieceData` _array_element_2)) (`local.TotalHeat`)))
      (switch `/Game/LD54/Blueprints/Structures/PieceType` _piecedata_piecetype_2
        (:`NewEnumerator1`
          (bind _returnvalue_2 (`KismetMathLibrary.FTrunc` (* (`local.TempBoost`) _piecedata_performance_2)))
          (set `local.CPU` (+ (`local.CPU`) _returnvalue_2))
          (set `local.CPUBoosted` (or (`local.CPUBoosted`) _returnvalue)))
        (:`NewEnumerator2`
          (set `local.GPU` (+ (`local.GPU`) _returnvalue_2))
          (set `local.GPUBoosted` (or (`local.GPUBoosted`) _returnvalue)))
        (:`NewEnumerator3`
          (set `local.RAM` (+ (`local.RAM`) _returnvalue_2))
          (set `local.RAMBoosted` (or (`local.RAMBoosted`) _returnvalue)))
        (:`NewEnumerator4`
          (set `local.MaxWatt` (+ (`local.MaxWatt`) _returnvalue_2))
          (set `local.MaxWattBoosted` (or (`local.MaxWattBoosted`) _returnvalue)))
        (:`NewEnumerator5`
          (set `local.DISK` (+ (`local.DISK`) _returnvalue_2))
          (set `local.DISKBoosted` (or (`local.DISKBoosted`) _returnvalue)))
        (:`NewEnumerator6`
          (set `local.TotalHeat` (+ (`local.TotalHeat`) _returnvalue_2))
          (set `local.HeatReducBoosted` (or (`local.HeatReducBoosted`) _returnvalue))))))
  (`/Game/LD54/Blueprints/UI/MachineStateUI/WBP_MachineState.UpdateMachineStateUI` (`self.MachineStateUI`) (`local.CPU`) (`self.GetRequirementForType` "NewEnumerator1") (`local.GPU`) (`self.GetRequirementForType` "NewEnumerator2") (`local.RAM`) (`self.GetRequirementForType` "NewEnumerator3") (`local.DISK`) (`self.GetRequirementForType` "NewEnumerator5") (`local.TotalHeat`) (`self.MaxHeat`) (`local.TotalWatt`) (`local.MaxWatt`) (`BlueprintMapLibrary.Map_IsNotEmpty` (`local.Motherboards`)) (`local.CPUBoosted`) (`local.GPUBoosted`) (`local.RAMBoosted`) (`local.DISKBoosted`) (`local.MaxWattBoosted`) (`local.HeatReducBoosted`))
  ;[1 1 1] Can Launch
  (for _array_element_3 _currentleveldata_requirements
    (switch `/Game/LD54/Blueprints/Structures/PieceType` (break `/Game/LD54/Blueprints/Structures/Requirement` _array_element_3)
      (:`NewEnumerator1`
        (if (< (`local.CPU`) (`.Performance_6_1EDF2D8E40A049E2705FFC901E1A8807` (break `/Game/LD54/Blueprints/Structures/Requirement` _array_element_3)))
          (bind _output_get (set `self.CanLaunch` false :!label _label))
          (`/Game/LD54/Blueprints/UI/LaunchUI/WBP_LaunchUI.SetCanLaunch` (`self.LaunchUI`) _output_get)
          (return)))
      (:`NewEnumerator2`
        (if (< (`local.GPU`) (`.Performance_6_1EDF2D8E40A049E2705FFC901E1A8807` (break `/Game/LD54/Blueprints/Structures/Requirement` _array_element_3)))
          (goto _label)))
      (:`NewEnumerator3`
        (if (< (`local.RAM`) (`.Performance_6_1EDF2D8E40A049E2705FFC901E1A8807` (break `/Game/LD54/Blueprints/Structures/Requirement` _array_element_3)))
          (goto _label)))
      (:`NewEnumerator5`
        (if (< (`local.DISK`) (`.Performance_6_1EDF2D8E40A049E2705FFC901E1A8807` (break `/Game/LD54/Blueprints/Structures/Requirement` _array_element_3)))
          (goto _label)))))
  (bind _output_get_2 (set `self.CanLaunch` (and (`BlueprintMapLibrary.Map_IsNotEmpty` (`local.Motherboards`)) (> (`local.CPU`) 0) (<= (`local.TotalHeat`) (`self.MaxHeat`)) (<= (`local.TotalWatt`) (`local.MaxWatt`)))))
  (`/Game/LD54/Blueprints/UI/LaunchUI/WBP_LaunchUI.SetCanLaunch` (`self.LaunchUI`) _output_get_2)
  (return))

(fn `RemovePiece`
  (params (PieceToRemove :type "/Game/LD54/Blueprints/BP_Piece Object Reference"))
  (`/Engine/EditorBlueprintResources/StandardMacros.IsValid` PieceToRemove
    (:`Is Valid`
      (`KismetArrayLibrary.Array_RemoveItem` (`self.Pieces`) PieceToRemove)
      (if (`/Game/LD54/Blueprints/BP_Piece.ValidPos` PieceToRemove)
        (`self.OnPieceChanged` null))
      (`self.K2_DestroyActor` PieceToRemove))))

(fn `SpawnCasing`
  (params (CasingData :type "/Game/LD54/Blueprints/Structures/CasingData Structure")))

(fn `SpawnNewPiece`
  (params (PieceData :type "/Game/LD54/Blueprints/Structures/PieceData Structure") (Location :type "Vector Structure"))
  (returns (NewPiece :type "/Game/LD54/Blueprints/BP_Piece Object Reference"))
  (bind _newpiece (`self.NewPiece`))
  (`/Engine/EditorBlueprintResources/StandardMacros.IsValid` _newpiece
    (:`Is Valid`
      (`self.K2_DestroyActor` _newpiece)
      (set `self.NewPiece` null))
    (:`Is Not Valid`
      _))
  (bind _returnvalue (`|SpawnActorFromClass` "/Game/LD54/Blueprints/BP_Piece.BP_Piece_C" (`KismetMathLibrary.MakeTransform` Location) "Undefined" "MultiplyWithRoot" null null))
  (`/Game/LD54/Blueprints/BP_Piece.SetPieceData` _returnvalue PieceData)
  (bind _output_get (set `self.NewPiece` _returnvalue))
  (return _output_get))

(fn `SpendMoney`
  (params (Price :type Integer))
  (bind _output_get (set `self.Balance` (- (`self.Balance`) Price)))
  (`/Game/LD54/Blueprints/UI/Eco/WBP_ECO.UpdateBalance` (`self.EcoUI`) _output_get))

(fn `StartLevel`
  (bind _currentlevelindex (`self.CurrentLevelIndex`))
  (bind _levels (`/Game/LD54/Data/LevelLib.Levels` (`self.LevelLib`)))
  ;[1 1 1] Hide Eco
  (`Widget.RemoveFromParent` (`self.EcoUI`))
  ;[1 1 1] LevelIncrement
  (bind _output_get (set `self.CurrentLevelIndex` (+ (`self.CurrentLevelIndex`) 1)))
  (`TextBlock.SetText` (`/Game/LD54/Blueprints/UI/BreakingNewsUI/WBP_BreakingNews.TextBlock_0` (`self.BreakingNewsUI`)) (`KismetTextLibrary.Conv_StringToText` (`KismetStringLibrary.Concat_StrStr` "Level " (`KismetStringLibrary.Conv_IntToString` (+ _output_get 1)))))
  (if (< _currentlevelindex (`KismetArrayLibrary.Array_Length` _levels))
    ;[1 1 1] Level
    (bind _output_get_2 (set `self.CurrentLevelData` (`|GetArrayItem` _levels _currentlevelindex)))
    ;[1 1 1] Casing
    (bind _returnvalue (`|SpawnActorFromClass` "/Game/LD54/Blueprints/BP_Casing.BP_Casing_C" (`KismetMathLibrary.MakeTransform` (0.0 -50.0 0.0)) "Undefined" "MultiplyWithRoot" null null))
    (`/Game/LD54/Blueprints/BP_Casing.SetCasingData` _returnvalue (break `/Game/LD54/Blueprints/Structures/LevelData` _output_get_2))
    (set `self.Casing` _returnvalue)
    ;[1 1 1] Update
    (`self.OnPieceChanged` null)
    (else
      (bind _returnvalue_2 (`|CreateWidget` "/Game/LD54/Blueprints/UI/gameend.gameend_C"))
      (`UserWidget.AddToViewport` _returnvalue_2 0))))

(fn `UserConstructionScript`)