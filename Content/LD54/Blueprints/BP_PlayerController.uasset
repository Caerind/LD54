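; Player controller for a PC-component placement puzzle, handling mouse drag, rotation and deletion of BP_Piece actors.
; Enhanced Input clicks pick the piece under the cursor, and Tick moves it by a stored offset on the Y=0 plane.
; Release places pieces at valid positions or restores their starting transform with an error sound.
; Rotation outside dragging reverts if it invalidates a valid position; deletion goes through the custom game mode.
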(event `self.ReceiveBeginPlay`
  (`EnhancedInputSubsystemInterface.AddMappingContext` (subsystem `EnhancedInputLocalPlayerSubsystem`) "/Game/LD54/Blueprints/Inputs/IMC_Default.IMC_Default" 0 (struct)))

(event `EnhancedInput|/Game/LD54/Blueprints/Inputs/INP_Click`
  (params (ActionValue :type Boolean) (ElapsedSeconds :type "Float (double-precision)") (TriggeredSeconds :type "Float (double-precision)") (InputAction :type "InputAction Object Reference" :default "/Game/LD54/Blueprints/Inputs/INP_Click.INP_Click"))
  (:`Started`
    (`self.StartDragAndDrop` (`self.GetPieceUnderCursor`)))
  (:`Canceled`
    (`self.StopDragAndDrop` :!label _label))
  (:`Completed`
    (goto _label)))

(event `EnhancedInput|/Game/LD54/Blueprints/Inputs/INP_RotateKey`
  (params (ActionValue :type Boolean) (ElapsedSeconds :type "Float (double-precision)") (TriggeredSeconds :type "Float (double-precision)") (InputAction :type "InputAction Object Reference" :default "/Game/LD54/Blueprints/Inputs/INP_RotateKey.INP_RotateKey"))
  (bind _selectedpiece (`self.SelectedPiece`))
  (:`Started`
    (`/Engine/EditorBlueprintResources/StandardMacros.IsValid` _selectedpiece
      (:`Is Valid`
        (`self.RotatePiece` _selectedpiece)))))

(event `EnhancedInput|/Game/LD54/Blueprints/Inputs/INP_DeleteKey`
  (params (ActionValue :type Boolean) (ElapsedSeconds :type "Float (double-precision)") (TriggeredSeconds :type "Float (double-precision)") (InputAction :type "InputAction Object Reference" :default "/Game/LD54/Blueprints/Inputs/INP_DeleteKey.INP_DeleteKey"))
  (bind _selectedpiece (`self.SelectedPiece`))
  (:`Started`
    (`/Engine/EditorBlueprintResources/StandardMacros.IsValid` _selectedpiece
      (:`Is Valid`
        (`self.RemovePiece` _selectedpiece)))))

(event `self.ReceiveTick`
  (params (DeltaSeconds :type "Float (single-precision)"))
  (bind _selectedpiece (`self.SelectedPiece`))
  (`/Engine/EditorBlueprintResources/StandardMacros.IsValid` _selectedpiece
    (:`Is Valid`
      (if (and (`self.DragAndDrop`) (`KismetSystemLibrary.IsValid` _selectedpiece))
        (`self.K2_SetActorLocation` _selectedpiece (+ (`self.DragAndDropOffset`) (`self.GetLocationUnderCursor`)) false true)))))

(event `EnhancedInput|/Game/LD54/Blueprints/Inputs/INP_DeleteMouse`
  (params (ActionValue :type Boolean) (ElapsedSeconds :type "Float (double-precision)") (TriggeredSeconds :type "Float (double-precision)") (InputAction :type "InputAction Object Reference" :default "/Game/LD54/Blueprints/Inputs/INP_DeleteMouse.INP_DeleteMouse"))
  (bind _pickedpiece (`self.GetPieceUnderCursor`))
  (:`Started`
    (`/Engine/EditorBlueprintResources/StandardMacros.IsValid` _pickedpiece
      (:`Is Valid`
        (`self.RemovePiece` _pickedpiece)))))

(fn `GetLocationUnderCursor`
  (returns (Location :type "Vector Structure"))
  (bind _worldlocation (`self.DeprojectMousePositionToWorld`))
  (return (`KismetMathLibrary.MakeVector` (.x _worldlocation) 0.0 (.z _worldlocation))))

(fn `GetPieceUnderCursor`
  (returns (PickedPiece :type "/Game/LD54/Blueprints/BP_Piece Object Reference"))
  (bind (_bblockinghit _binitialoverlap _time _distance _location _impactpoint _normal _impactnormal _physmat _hitactor) (`GameplayStatics.BreakHitResult` (`self.GetHitResultUnderCursorByChannel` "TraceTypeQuery1" false)))
  (if _bblockinghit
    (bind _asbp_piece (cast `/Game/LD54/Blueprints/BP_Piece` _hitactor)
      (:`then`
        (return _asbp_piece))
      (:`CastFailed`
        _)))
  (return null))

(fn `RemovePiece`
  (params (Piece :type "/Game/LD54/Blueprints/BP_Piece Object Reference"))
  (`/Engine/EditorBlueprintResources/StandardMacros.IsValid` Piece
    (:`Is Valid`
      (if (== Piece (`self.SelectedPiece`))
        (set `self.SelectedPiece` null))
      (bind _gamemode (`/Game/LD54/Blueprints/BPL_Game.GetCustomGameMode` self))
      (`/Game/LD54/Blueprints/BP_GameMode.RemovePiece` _gamemode Piece)
      (`GameplayStatics.SpawnSound2D` "/Game/LD54/Sound/SoundCue/ControlSound/Destroy_Cue.Destroy_Cue" 1.0 1.0 0.0 null))))

(fn `RotatePiece`
  (params (Piece :type "/Game/LD54/Blueprints/BP_Piece Object Reference"))
  (locals (WasValid :type Boolean) (PreviousRotation :type "Rotator Structure"))
  (bind _selectedpiece (`self.SelectedPiece`))
  (bind _selectedpiece_2 (`self.SelectedPiece`))
  (if (`KismetSystemLibrary.IsValid` (`self.SelectedPiece`))
    (`GameplayStatics.SpawnSound2D` "/Game/LD54/Sound/SoundCue/ControlSound/Rotate_Cue.Rotate_Cue" 1.0 1.0 0.0 null)
    (bind _validpos (`/Game/LD54/Blueprints/BP_Piece.CheckValidPos` _selectedpiece))
    (set `local.WasValid` _validpos)
    (set `local.PreviousRotation` (`self.K2_GetActorRotation` _selectedpiece))
    (`self.K2_SetActorRotation` (`self.SelectedPiece`) (`KismetMathLibrary.ComposeRotators` (`local.PreviousRotation`) (struct :`Pitch` -90.0)) false)
    ;[1 1 1] Early return if dd
    (if (`self.DragAndDrop`)
      (return)
      (else
        ;[1 1 1] Otherwise check if previous was valid and not now
        (bind _validpos_2 (`/Game/LD54/Blueprints/BP_Piece.CheckValidPos` _selectedpiece_2))
        (if (and (`local.WasValid`) (not _validpos_2))
          (`self.K2_SetActorRotation` _selectedpiece_2 (`local.PreviousRotation`) false))
        (return)))))

(fn `StartDragAndDrop`
  (params (Piece :type "/Game/LD54/Blueprints/BP_Piece Object Reference"))
  (bind _returnvalue (`self.K2_GetActorLocation` Piece))
  (bind _selectedpiece (`self.SelectedPiece`))
  (if (and (!= Piece _selectedpiece) (`KismetSystemLibrary.IsValid` _selectedpiece))
    (set `/Game/LD54/Blueprints/BP_Piece.Selected` false _selectedpiece)
    (set `self.SelectedPiece` null))
  (`/Engine/EditorBlueprintResources/StandardMacros.IsValid` Piece
    (:`Is Valid`
      (set `self.DragAndDrop` true)
      (set `self.DragAndDropStartPos` _returnvalue)
      (set `self.DragAndDropOffset` (- _returnvalue (`self.GetLocationUnderCursor`)))
      (set `self.DragAndDropStartRotation` (`self.K2_GetActorRotation` Piece))
      (bind _output_get (set `self.SelectedPiece` Piece))
      (set `/Game/LD54/Blueprints/BP_Piece.Selected` true _output_get)
      (`GameplayStatics.SpawnSound2D` "/Game/LD54/Sound/SoundCue/ControlSound/ComponentDrag_Cue.ComponentDrag_Cue" 1.0 1.0 0.0 null))
    (:`Is Not Valid`
      (return))))

(fn `StopDragAndDrop`
  (bind _selectedpiece (`self.SelectedPiece`))
  (bind _selectedpiece_2 (`self.SelectedPiece`))
  (bind _selectedpiece_3 (`self.SelectedPiece`))
  (bind _selectedpiece_4 (`self.SelectedPiece`))
  (bind (_piecedata_name _piecedata_vendor _piecedata_piecetype) (break `/Game/LD54/Blueprints/Structures/PieceData` (`/Game/LD54/Blueprints/BP_Piece.PieceData` _selectedpiece_2)))
  (if (and (`self.DragAndDrop`) (`KismetSystemLibrary.IsValid` _selectedpiece_4))
    (if (`/Game/LD54/Blueprints/BP_Piece.ValidPos` _selectedpiece_4)
      (`/Game/LD54/Blueprints/BP_Piece.OnPlace` _selectedpiece_4)
      (set `self.DragAndDrop` false)
      (`/Engine/EditorBlueprintResources/StandardMacros.IsValid` _selectedpiece_2
        (:`Is Valid`
          (set `/Game/LD54/Blueprints/BP_Piece.Selected` false _selectedpiece_2)
          (switch `/Game/LD54/Blueprints/Structures/PieceType` _piecedata_piecetype
            (:`NewEnumerator0`
              _)
            (:`NewEnumerator1`
              _)
            (:`NewEnumerator2`
              _)
            (:`NewEnumerator3`
              _)
            (:`NewEnumerator4`
              _)
            (:`NewEnumerator5`
              _)
            (:`NewEnumerator6`
              _))
          (`GameplayStatics.SpawnSound2D` "/Game/LD54/Sound/SoundCue/ControlSound/ComponentDrop_Cue.ComponentDrop_Cue" 1.0 1.0 0.0 null)
          (set `self.SelectedPiece` null)))
      (else
        (`self.K2_SetActorLocation` _selectedpiece_4 (`self.DragAndDropStartPos`) false true)
        (`self.K2_SetActorRotation` _selectedpiece_4 (`self.DragAndDropStartRotation`) true)
        (set `self.DragAndDrop` false)
        (`/Engine/EditorBlueprintResources/StandardMacros.IsValid` _selectedpiece_3
          (:`Is Valid`
            (`GameplayStatics.SpawnSound2D` "/Game/LD54/Sound/SoundCue/ErrorSound_Cue.ErrorSound_Cue" 1.0 1.0 0.0 null)
            (set `/Game/LD54/Blueprints/BP_Piece.Selected` false _selectedpiece_3)
            (set `self.SelectedPiece` null)))))
    (else
      (set `self.DragAndDrop` false)
      (`/Engine/EditorBlueprintResources/StandardMacros.IsValid` _selectedpiece
        (:`Is Valid`
          (set `/Game/LD54/Blueprints/BP_Piece.Selected` false _selectedpiece)
          (set `self.SelectedPiece` null))))))

(fn `UserConstructionScript`)