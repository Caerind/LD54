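; BP_Piece is a placeable 2D puzzle piece that fits onto a 16-unit grid inside the game mode's Casing.
; SetPieceData applies the sprite and offsets a Start anchor, from which PieceShape cells map through the transform to grid coordinates.
; While selected, Tick checks every cell against the Casing to update ValidPos.
; OnPlace snaps by the first cell, box-traces to remove pieces sharing a cell, then notifies the game mode.
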(event `self.ReceiveTick`
  (params (DeltaSeconds :type "Float (single-precision)"))
  (if (`self.Selected`)
    (`self.CheckValidPos`)))

(fn `CheckValidPos`
  (returns (ValidPos :type Boolean))
  (bind (_piecedata_name _piecedata_vendor _piecedata_piecetype _piecedata_pieceshape) (break `/Game/LD54/Blueprints/Structures/PieceData` (`self.PieceData`)))
  (for _array_element _piecedata_pieceshape
    (bind _gamemode (`/Game/LD54/Blueprints/BPL_Game.GetCustomGameMode` self))
    (bind (_x _y) (break `/Game/LD54/Blueprints/Structures/Vector2Int` _array_element))
    (bind _valid (`/Game/LD54/Blueprints/BP_Casing.IsValidCasingPos` (`/Game/LD54/Blueprints/BP_GameMode.Casing` _gamemode) (`KismetMathLibrary.Round` (/ (.x (`KismetMathLibrary.TransformLocation` (`SceneComponent.K2_GetComponentToWorld` (`self.Start`)) (`KismetMathLibrary.MakeVector` (`KismetMathLibrary.Conv_IntToDouble` (* _x 16)) 0.0 (`KismetMathLibrary.Conv_IntToDouble` (* _y -16))))) 16.0)) (`KismetMathLibrary.Round` (/ (.z (`KismetMathLibrary.TransformLocation` (`SceneComponent.K2_GetComponentToWorld` (`self.Start`)) (`KismetMathLibrary.MakeVector` (`KismetMathLibrary.Conv_IntToDouble` (* _x 16)) 0.0 (`KismetMathLibrary.Conv_IntToDouble` (* _y -16))))) 16.0))))
    (if (not _valid)
      (bind _output_get (set `self.ValidPos` false))
      (return _output_get)))
  (bind _output_get_2 (set `self.ValidPos` true))
  (return _output_get_2))

(fn `OnPlace`
  (locals (TempRemovePiece :type Boolean))
  (bind (_piecedata_name _piecedata_vendor _piecedata_piecetype _piecedata_pieceshape) (break `/Game/LD54/Blueprints/Structures/PieceData` (`self.PieceData`)))
  (bind _gamemode (`/Game/LD54/Blueprints/BPL_Game.GetCustomGameMode` self))
  (for (_array_element _array_index) _piecedata_pieceshape
    (if (== _array_index 0)
      (bind (_x _y) (break `/Game/LD54/Blueprints/Structures/Vector2Int` _array_element))
      (bind _returnvalue (`KismetMathLibrary.TransformLocation` (`SceneComponent.K2_GetComponentToWorld` (`self.Start`)) (`KismetMathLibrary.MakeVector` (`KismetMathLibrary.Conv_IntToDouble` (* _x 16)) 0.0 (`KismetMathLibrary.Conv_IntToDouble` (* _y -16)))))
      ;[1 1 1] Round
      (`self.K2_SetActorLocation` (+ (- (`KismetMathLibrary.MakeVector` (* (`KismetMathLibrary.Round` (/ (.x _returnvalue) 16.0)) 16) 0.0 (* (`KismetMathLibrary.Round` (/ (.z _returnvalue) 16.0)) 16)) _returnvalue) (`self.K2_GetActorLocation`)) false true))
    (bind (_outhit _returnvalue_2) (`KismetSystemLibrary.BoxTraceSingle` _returnvalue _returnvalue (6.0 6.0 6.0) (struct) "TraceTypeQuery1" true))
    (if _returnvalue_2
      (bind _asbp_piece (cast `/Game/LD54/Blueprints/BP_Piece` (`.HitActor` (`GameplayStatics.BreakHitResult` _outhit))))
      (set `local.TempRemovePiece` false)
      (bind (_piecedata_name_2 _piecedata_vendor_2 _piecedata_piecetype_2 _piecedata_pieceshape_2) (break `/Game/LD54/Blueprints/Structures/PieceData` (`/Game/LD54/Blueprints/BP_Piece.PieceData` _asbp_piece)))
      (for _array_element_2 _piecedata_pieceshape_2
        (bind (_x_2 _y_2) (break `/Game/LD54/Blueprints/Structures/Vector2Int` _array_element_2))
        (if (and (== (`KismetMathLibrary.Round` (/ (.x (`KismetMathLibrary.TransformLocation` (`SceneComponent.K2_GetComponentToWorld` (`/Game/LD54/Blueprints/BP_Piece.Start` _asbp_piece)) (`KismetMathLibrary.MakeVector` (`KismetMathLibrary.Conv_IntToDouble` (* _x_2 16)) 0.0 (`KismetMathLibrary.Conv_IntToDouble` (* _y_2 -16))))) 16.0)) (`KismetMathLibrary.Round` (/ (.x _returnvalue) 16.0))) (== (`KismetMathLibrary.Round` (/ (.z (`KismetMathLibrary.TransformLocation` (`SceneComponent.K2_GetComponentToWorld` (`/Game/LD54/Blueprints/BP_Piece.Start` _asbp_piece)) (`KismetMathLibrary.MakeVector` (`KismetMathLibrary.Conv_IntToDouble` (* _x_2 16)) 0.0 (`KismetMathLibrary.Conv_IntToDouble` (* _y_2 -16))))) 16.0)) (`KismetMathLibrary.Round` (/ (.z _returnvalue) 16.0))))
          (set `local.TempRemovePiece` true)))
      (if (`local.TempRemovePiece`)
        (`/Game/LD54/Blueprints/BP_GameMode.RemovePiece` _gamemode _asbp_piece))))
  (`/Game/LD54/Blueprints/BP_GameMode.OnPieceChanged` _gamemode self))

(fn `SetPieceData`
  (params (PieceData :type "/Game/LD54/Blueprints/Structures/PieceData Structure"))
  (bind (_origin _boxextent) (`self.GetActorBounds` false))
  (bind _papersprite (`self.PaperSprite`))
  (bind _returnvalue (* (.x _boxextent) -1.0))
  (bind _output_get (set `self.PieceData` PieceData))
  (`PaperSpriteComponent.SetSprite` _papersprite (`.Sprite_31_4F0C128E473A9AF05CFF77998CA2ED32` (break `/Game/LD54/Blueprints/Structures/PieceData` _output_get)))
  (`SceneComponent.K2_SetRelativeLocation` _papersprite (`KismetMathLibrary.MakeVector` _returnvalue 0.0 (.z _boxextent)) false false)
  (`SceneComponent.K2_SetRelativeLocation` (`self.Start`) (`KismetMathLibrary.MakeVector` (+ _returnvalue 8.0) 0.0 (+ (.z _boxextent) -8.0)) false false))

(fn `UserConstructionScript`)