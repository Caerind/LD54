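; BP_Casing is a tile-map casing whose layout comes from the shape stored in its casing data.
; SetCasingData stores that data, adds a layer to the Paper2D tile map, paints a tile at each shape coordinate and rebuilds collision.
; IsValidCasingPos linearly searches the shape to report whether a position lies inside it, negating the queried Y before comparing with the stored coordinates.
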(fn `IsValidCasingPos`
  (params (X :type Integer) (Y :type Integer))
  (returns (Valid :type Boolean))
  (bind _casingdata_shape (break `/Game/LD54/Blueprints/Structures/CasingData` (`self.CasingData`)))
  (for _array_element _casingdata_shape
    (if (and (== (break `/Game/LD54/Blueprints/Structures/Vector2Int` _array_element) X) (== (- 0 Y) (`.Y_5_0D42DD4D4E9BE49F6D4235832CC2E4DC` (break `/Game/LD54/Blueprints/Structures/Vector2Int` _array_element))))
      (return true)))
  (return false))

(fn `SetCasingData`
  (params (CasingData :type "/Game/LD54/Blueprints/Structures/CasingData Structure"))
  (bind _papertilemap (`self.PaperTileMap`))
  (`PaperTileMapComponent.AddNewLayer` _papertilemap)
  (bind _output_get (set `self.CasingData` CasingData))
  (for _array_element (break `/Game/LD54/Blueprints/Structures/CasingData` _output_get)
    (`PaperTileMapComponent.SetTile` _papertilemap (break `/Game/LD54/Blueprints/Structures/Vector2Int` _array_element) (`.Y_5_0D42DD4D4E9BE49F6D4235832CC2E4DC` (break `/Game/LD54/Blueprints/Structures/Vector2Int` _array_element)) 0 (`self.PaperTileInfo`)))
  (`PaperTileMapComponent.SetLayerCollision` _papertilemap 0 true true 50.0 false 0.0 true)
  (`PaperTileMapComponent.RebuildCollision` _papertilemap)
  (return))

(fn `UserConstructionScript`)